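; Checkpoint actor for the Time Attack mode that detects when a TimeAttackPawn passes through it in the correct direction.
; On trigger end overlap, a dot product of pawn velocity and the Arrow's forward vector must be positive.
; A valid pass fires the CheckpointPassed dispatcher with the checkpoint's index, then deactivates it.
; Activate and Deactivate toggle the particle and trigger visibility along with the trigger's overlap events.
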(event `self.Trigger.OnComponentEndOverlap`
  (params (OverlappedComponent :type "PrimitiveComponent Object Reference") (OtherActor :type "Actor Object Reference") (OtherComp :type "PrimitiveComponent Object Reference") (OtherBodyIndex :type Integer))
  (bind _astime_attack_pawn (cast `TimeAttackPawn` OtherActor))
  (if (> (`KismetMathLibrary.Dot_VectorVector` (`self.GetVelocity` _astime_attack_pawn) (`KismetMathLibrary.Conv_RotatorToVector` (`SceneComponent.K2_GetComponentRotation` (`self.Arrow`)))) 0.0)
    (`self.CheckpointPassed` (`self.CheckpointIndex`))
    (`self.Deactivate`)))

(fn `Activate`
  (bind _trigger (`self.Trigger`))
  (`SceneComponent.SetHiddenInGame` (`self.ParticleSystem`) false false)
  (`SceneComponent.SetHiddenInGame` _trigger false false)
  (set `PrimitiveComponent.bGenerateOverlapEvents` true _trigger))

(fn `Deactivate`
  (bind _trigger (`self.Trigger`))
  (`SceneComponent.SetHiddenInGame` (`self.ParticleSystem`) true false)
  (`SceneComponent.SetHiddenInGame` _trigger true false)
  (set `PrimitiveComponent.bGenerateOverlapEvents` false _trigger))

(fn `UserConstructionScript`)